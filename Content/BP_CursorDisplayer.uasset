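; Tutorial Blueprint on object references and casting, which prints the random number of the BP_RandomGenerator under the mouse cursor.
; Tick traces under the cursor on Visibility, casts the hit actor to BP_RandomGenerator and stores it.
; BeginPlay shows the cursor and caches the cast game mode to avoid per-frame casting; UpdateBCount zeroes its BananaGM through that reference.
; Unconnected numbered step chains preserve earlier lesson stages.
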(event `self.ReceiveTick`
  (params (DeltaSeconds :type "Float (single-precision)"))
  ;[1 1 1] Step5
  ; Now we can cast to verify the class AND
  ; Save the dynamic object in a variable AND
  ; get access to the BP_random Genereator Content
  (set `self.BP_RandomGenRef` null) ; optonal: clear variable
  (bind _hitactorref (`self.GetActorUnderCursor`))
  (bind _output_get (set `self.Actor` _hitactorref))
  (bind _asbp_random_generator (cast `/Game/BP_RandomGenerator` _output_get))
  (set `self.BP_RandomGenRef` _asbp_random_generator)
  (`KismetSystemLibrary.PrintString` (`KismetStringLibrary.Concat_StrStr` "Random number is:" (`KismetStringLibrary.Conv_IntToString` (`/Game/BP_RandomGenerator.RandomNumber` (`self.BP_RandomGenRef`)))) true true (struct :`G` 0.66 :`B` 1.0 :`A` 1.0) 0.0))

(event `self.ReceiveBeginPlay`
  (set `PlayerController.bShowMouseCursor` true (`GameplayStatics.GetPlayerController` 0))
  ;[1 1 1] Since a cast every frame is very expensive that's why we do it in the begin play, save the object and use it later
  (bind _asbp_first_person_game_mode (cast `/Game/FirstPerson/Blueprints/BP_FirstPersonGameMode` (`GameplayStatics.GetGameMode`)))
  (set `self.As BP First Person Game Mode` _asbp_first_person_game_mode))

(event `UpdateBCount`
  ;[1 1 1] Since a cast every frame is very expensive that's why we do it in the begin play, save the object and use it later
  (set `/Game/FirstPerson/Blueprints/BP_FirstPersonGameMode.BananaGM` 0 (`self.As BP First Person Game Mode`)))

(fn `GetActorUnderCursor`
  (returns (HitActorRef :type "Actor Object Reference"))
  (return (`.HitActor` (`GameplayStatics.BreakHitResult` (`PlayerController.GetHitResultUnderCursorByChannel` (`GameplayStatics.GetPlayerController` 0) "TraceTypeQuery1" true)))))

(fn `UserConstructionScript`)