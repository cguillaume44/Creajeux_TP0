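; BP_Banana is an actor that counts hits on its Cube and shows the total on its Counter text.
; On BeginPlay it stores a reference to itself in BP_FirstPersonGameMode's BananaRef.
; Each component hit calls IncreaseBanana to increment CountBanana and refresh the text.
; ResetBanana sets the count to a supplied value and updates the display, though nothing in this file calls it.
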(event `self.ReceiveBeginPlay`
  (bind _asbp_first_person_game_mode (cast `/Game/FirstPerson/Blueprints/BP_FirstPersonGameMode` (`GameplayStatics.GetGameMode`)))
  (set `/Game/FirstPerson/Blueprints/BP_FirstPersonGameMode.BananaRef` self _asbp_first_person_game_mode))

(event `self.Cube.OnComponentHit`
  (params (HitComponent :type "PrimitiveComponent Object Reference") (OtherActor :type "Actor Object Reference") (OtherComp :type "PrimitiveComponent Object Reference") (NormalImpulse :type "Vector Structure") (Hit :type "HitResult Structure (by ref)"))
  (`self.Increase Banana`))

(fn `Increase Banana`
  (bind _result (`/Engine/EditorBlueprintResources/StandardMacros.IncrementInt` (`self.CountBanana`))
    (:`  `
      (`TextRenderComponent.K2_SetText` (`self.Counter`) (`KismetTextLibrary.Conv_IntToText` _result)))))

(fn `ResetBanana`
  (params (CountBanana :type Integer))
  (bind _output_get (set `self.CountBanana` CountBanana))
  (`TextRenderComponent.K2_SetText` (`self.Counter`) (`KismetTextLibrary.Conv_IntToText` _output_get)))

(fn `UserConstructionScript`)