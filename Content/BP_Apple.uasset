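; BP_Apple is an actor that counts hits on its Cube component and shows the total on its Counter text.
; On BeginPlay it stores a reference to itself in BP_FirstPersonGameMode.
; Any component hit on the Cube calls IncreaseApple to increment CountApple and refresh the text.
; ResetApple sets the count to a supplied value and updates the display.
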(event `self.ReceiveBeginPlay`
  (bind _asbp_first_person_game_mode (cast `/Game/FirstPerson/Blueprints/BP_FirstPersonGameMode` (`GameplayStatics.GetGameMode`)))
  (set `/Game/FirstPerson/Blueprints/BP_FirstPersonGameMode.AppleRef` self _asbp_first_person_game_mode))

(event `self.Cube.OnComponentHit`
  (params (HitComponent :type "PrimitiveComponent Object Reference") (OtherActor :type "Actor Object Reference") (OtherComp :type "PrimitiveComponent Object Reference") (NormalImpulse :type "Vector Structure") (Hit :type "HitResult Structure (by ref)"))
  (`self.Increase Apple`))

(fn `Increase Apple`
  (bind _result (`/Engine/EditorBlueprintResources/StandardMacros.IncrementInt` (`self.CountApple`))
    (:`  `
      (set `self.TextApple` (`KismetTextLibrary.Conv_IntToText` _result))
      (`TextRenderComponent.K2_SetText` (`self.Counter`) (`self.TextApple`)))))

(fn `ResetApple`
  (params (CountApple :type Integer))
  (bind _output_get (set `self.CountApple` CountApple))
  (set `self.TextApple` (`KismetTextLibrary.Conv_IntToText` _output_get))
  (`TextRenderComponent.K2_SetText` (`self.Counter`) (`self.TextApple`)))

(fn `UserConstructionScript`)